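; Ritual is a collectible pickup that counts toward a total displayed out of five.
; Overlapping its interaction area registers it on BP_FirstPersonCharacter as the interactable ritual unless already taken, and leaving clears that reference.
; Hide, not called within this Blueprint, makes it invisible, marks it taken, increments the player's collected count, shows Turkish progress text and plays a pickup sound.
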(event OnComponentBeginOverlap(InteractionArea)
  (params (OverlappedComponent :type Primitive%20Component%20Object%20Reference) (OtherActor :type Actor%20Object%20Reference) (OtherComp :type Primitive%20Component%20Object%20Reference) (OtherBodyIndex :type Integer) (bFromSweep :type Boolean) (SweepResult :type Hit%20Result%20Structure%20%28by%20ref%29))
  (bind _asbp_first_person_character (Utilities|Casting|CastToBP_FirstPersonCharacter OtherActor))
  (if (not (Variables|Default|GetTaken))
    (Variables|/Game/Konya/Blueprints/BP_FirstPersonCharacter.BP_FirstPersonCharacter_C|SetInteracting _asbp_first_person_character true)
    (Variables|/Game/Konya/Blueprints/BP_FirstPersonCharacter.BP_FirstPersonCharacter_C|SetInteracted%20Ritual _asbp_first_person_character self)))

(event OnComponentEndOverlap(InteractionArea)
  (params (OverlappedComponent :type Primitive%20Component%20Object%20Reference) (OtherActor :type Actor%20Object%20Reference) (OtherComp :type Primitive%20Component%20Object%20Reference) (OtherBodyIndex :type Integer))
  (bind _asbp_first_person_character (Utilities|Casting|CastToBP_FirstPersonCharacter OtherActor))
  (Variables|/Game/Konya/Blueprints/BP_FirstPersonCharacter.BP_FirstPersonCharacter_C|SetInteracting _asbp_first_person_character false)
  (Variables|/Game/Konya/Blueprints/BP_FirstPersonCharacter.BP_FirstPersonCharacter_C|SetInteracted%20Ritual _asbp_first_person_character 0))

(fn ConstructionScript)

(fn Hide
  (Rendering|SetVisibility (Variables|Default|GetDefaultSceneRoot) false true)
  (Variables|Default|SetTaken true)
  (bind _asbp_first_person_character (Utilities|Casting|CastToBP_FirstPersonCharacter (Game|GetPlayerCharacter 0)))
  (bind _output_get (Variables|/Game/Konya/Blueprints/BP_FirstPersonCharacter.BP_FirstPersonCharacter_C|SetCollected%20Rituals _asbp_first_person_character (+ (Variables|/Game/Konya/Blueprints/BP_FirstPersonCharacter.BP_FirstPersonCharacter_C|GetCollected%20Rituals _asbp_first_person_character) 1)))
  (Default|ShowText _asbp_first_person_character (Utilities|String|BuildString(Integer) "Toplamda bulunan ritüeller " "" _output_get "/5") false)
  (Audio|PlaySound2D "/Game/Konya/Audio/Ritual_Picked.Ritual_Picked" 7.0 1.0 0.0 0 _asbp_first_person_character))