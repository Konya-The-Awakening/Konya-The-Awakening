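; LayingMan is a corpse item that the first-person player can set on fire.
; Its collision box sets the player's CanFireCorpse flag on overlap begin and clears it on overlap end.
; SetFire toggles the fire animation's visibility, clears that flag on the player character and latches Fired once lit.
; The overlap events do not check Fired, so re-entering the box sets CanFireCorpse again.
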(event OnComponentBeginOverlap(CollisionBox)
  (params (OverlappedComponent :type Primitive%20Component%20Object%20Reference) (OtherActor :type Actor%20Object%20Reference) (OtherComp :type Primitive%20Component%20Object%20Reference) (OtherBodyIndex :type Integer) (bFromSweep :type Boolean) (SweepResult :type Hit%20Result%20Structure%20%28by%20ref%29))
  (bind _asbp_first_person_character (Utilities|Casting|CastToBP_FirstPersonCharacter OtherActor))
  (Variables|/Game/Konya/Blueprints/BP_FirstPersonCharacter.BP_FirstPersonCharacter_C|SetCan%20Fire%20Corpse _asbp_first_person_character true))

(event OnComponentEndOverlap(CollisionBox)
  (params (OverlappedComponent :type Primitive%20Component%20Object%20Reference) (OtherActor :type Actor%20Object%20Reference) (OtherComp :type Primitive%20Component%20Object%20Reference) (OtherBodyIndex :type Integer))
  (bind _asbp_first_person_character (Utilities|Casting|CastToBP_FirstPersonCharacter OtherActor))
  (Variables|/Game/Konya/Blueprints/BP_FirstPersonCharacter.BP_FirstPersonCharacter_C|SetCan%20Fire%20Corpse _asbp_first_person_character false))

(fn ConstructionScript)

(fn SetFire
  (params (Fire :type Boolean))
  (Rendering|SetVisibility (Variables|Components|GetFire%20Animation) Fire false)
  (bind _asbp_first_person_character (Utilities|Casting|CastToBP_FirstPersonCharacter (Game|GetPlayerCharacter 0)))
  (Variables|/Game/Konya/Blueprints/BP_FirstPersonCharacter.BP_FirstPersonCharacter_C|SetCan%20Fire%20Corpse _asbp_first_person_character false)
  (if Fire
    (Variables|Default|SetFired true)))