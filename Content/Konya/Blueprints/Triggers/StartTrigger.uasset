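; StartTrigger is a one-shot overlap trigger that kicks off play by giving the player the objective of finding five rituals and the exit.
; The first overlap by any actor shows the Turkish hint text on the player's first-person character, makes HidableWall visible and calls RandomRoam on every BP_AI_IMAM.
; The construction script binds the wall automatically, taking the first HidableWall actor it finds in the level.
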(event Collision|EventActorBeginOverlap
  (params (OtherActor :type Actor%20Object%20Reference))
  (Utilities|FlowControl|DoOnce false
    (:Completed
      (bind _asbp_first_person_character (Utilities|Casting|CastToBP_FirstPersonCharacter (Game|GetPlayerCharacter 0)))
      (Default|ShowTextat _asbp_first_person_character "5 ritüel bul ve çıkışı yolunu ara..." "(X=750.000000,Y=900.000000)")
      (Default|SetVisibility (Variables|Default|GetHidable%20Wall) true)
      (bind _outactors (Actor|GetAllActorsOfClass "/Game/Konya/AI/Blueprints/BP_AI_IMAM.BP_AI_IMAM_C"))
      (for _array_element _outactors
        (Default|RandomRoam _array_element)))))

(fn ConstructionScript
  (bind _outactors (Actor|GetAllActorsOfClass "/Game/Konya/Blueprints/Items/HidableWall.HidableWall_C"))
  (Variables|Default|SetHidable%20Wall (Utilities|Array|Get(acopy) _outactors)))