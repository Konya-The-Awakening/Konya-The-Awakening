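; Lighter pickup actor that the first-person player character can collect.
; Overlapping its interaction area shows an interact widget, unless already taken, and registers the lighter on the character; leaving clears both.
; Collect hides the actor, marks it taken, shows a pickup message and sets the character's HasLighter flag.
; SetMesh swaps the static mesh between lit and unlit versions.
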(event OnComponentBeginOverlap(InteractionArea)
  (params (OverlappedComponent :type Primitive%20Component%20Object%20Reference) (OtherActor :type Actor%20Object%20Reference) (OtherComp :type Primitive%20Component%20Object%20Reference) (OtherBodyIndex :type Integer) (bFromSweep :type Boolean) (SweepResult :type Hit%20Result%20Structure%20%28by%20ref%29))
  (bind _asbp_first_person_character (Utilities|Casting|CastToBP_FirstPersonCharacter OtherActor))
  (if (not (Variables|Default|GetTaken))
    (Rendering|SetVisibility (Variables|Default|GetInteract%20Widget) true false)
    (Variables|/Game/Konya/Blueprints/BP_FirstPersonCharacter.BP_FirstPersonCharacter_C|SetLighter _asbp_first_person_character self)
    (Variables|/Game/Konya/Blueprints/BP_FirstPersonCharacter.BP_FirstPersonCharacter_C|SetInteracting%20With%20Lighter _asbp_first_person_character true)))

(event OnComponentEndOverlap(InteractionArea)
  (params (OverlappedComponent :type Primitive%20Component%20Object%20Reference) (OtherActor :type Actor%20Object%20Reference) (OtherComp :type Primitive%20Component%20Object%20Reference) (OtherBodyIndex :type Integer))
  (bind _asbp_first_person_character (Utilities|Casting|CastToBP_FirstPersonCharacter OtherActor))
  (Rendering|SetVisibility (Variables|Default|GetInteract%20Widget) false false)
  (Variables|/Game/Konya/Blueprints/BP_FirstPersonCharacter.BP_FirstPersonCharacter_C|SetLighter _asbp_first_person_character 0)
  (Variables|/Game/Konya/Blueprints/BP_FirstPersonCharacter.BP_FirstPersonCharacter_C|SetInteracting%20With%20Lighter _asbp_first_person_character false))

(event EventBeginPlay)

(event Collision|EventActorBeginOverlap
  (params (OtherActor :type Actor%20Object%20Reference)))

(event EventTick
  (params (DeltaSeconds :type Float%20%28single-precision%29)))

(fn ConstructionScript)

(fn Collect
  (Rendering|SetVisibility (Variables|Default|GetDefaultSceneRoot) false true)
  (Variables|Default|SetTaken true)
  (bind _asbp_first_person_character (Utilities|Casting|CastToBP_FirstPersonCharacter (Game|GetPlayerCharacter 0)))
  (Default|ShowText _asbp_first_person_character "You have picked up a lighter!" false)
  (Variables|/Game/Konya/Blueprints/BP_FirstPersonCharacter.BP_FirstPersonCharacter_C|SetHas%20Lighter _asbp_first_person_character true)
  (Variables|/Game/Konya/Blueprints/BP_FirstPersonCharacter.BP_FirstPersonCharacter_C|SetInteracting%20With%20Lighter _asbp_first_person_character false))

(fn SetMesh
  (params (Activated :type Boolean))
  (bind _staticmesh (Variables|Default|GetStaticMesh))
  (if Activated
    (Components|StaticMesh|SetStaticMesh _staticmesh "/Game/Konya/Meshes/LighterOn.LighterOn")
    (else
      (Components|StaticMesh|SetStaticMesh _staticmesh "/Game/Konya/Meshes/LighterOff.LighterOff"))))