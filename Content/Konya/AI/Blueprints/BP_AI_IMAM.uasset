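; BP_AI_IMAM is a roaming horror enemy that chases and jumpscares the first-person player.
; Pawn sensing starts the chase with sound, and a retriggerable delay resumes recursive random roaming once sightings stop.
; Within catch range it moves the player to its start transform, plays the jumpscare and applies damage, leading to death or checkpoint respawn.
; AI Perception stimuli send it to investigate the sensed location, and DoOnce gates prevent repeated triggers.
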(event OnSeePawn(PawnSensing)
  (params (Pawn :type Pawn%20Object%20Reference))
  (bind _self self)
  (bind _asbp_first_person_character (Utilities|Casting|CastToBP_FirstPersonCharacter Pawn))
  (Utilities|FlowControl|Sequence
    (:then_0
      (AI|AIMoveTo _self "0, 0, 0" _asbp_first_person_character 5.0 false
        (:then
          (if (< (Transformation|GetDistanceTo _self _asbp_first_person_character) 3e+02)
            (Utilities|FlowControl|DoOnce false :!label _label
              (:Completed
                (Audio|Components|Audio|Stop (Variables|Default|GetAudio%20Component))
                (Input|DisableInput _asbp_first_person_character 0)
                (Audio|PlaySound2D "/Game/Konya/Audio/Jumpscare.Jumpscare" 1.0 1.0 0.0 0 0)
                (Transformation|SetActorTransform _asbp_first_person_character (Variables|Default|GetStart%20Location))
                (Rendering|SetVisibility (Variables|/Game/Konya/Blueprints/BP_FirstPersonCharacter.BP_FirstPersonCharacter_C|GetJump%20Scare%20Mesh _asbp_first_person_character) true false)
                (Components|Animation|PlayAnimation (Variables|/Game/Konya/Blueprints/BP_FirstPersonCharacter.BP_FirstPersonCharacter_C|GetJump%20Scare%20Mesh _asbp_first_person_character) "/Game/Konya/AI/Animations/İmam/JumpScare.JumpScare" false)
                (Utilities|FlowControl|Delay 1.3)
                (bind _dead (Default|DoDamage _asbp_first_person_character))
                (if _dead
                  (Default|ShowDeadScreenandRestart _asbp_first_person_character)
                  (else
                    (bind _returnvalue (UserInterface|CreateWidget "/Game/Konya/Blueprints/UI/RespawnLoadingScreen.RespawnLoadingScreen_C"))
                    (UserInterface|Viewport|AddtoViewport _returnvalue 0)
                    (Utilities|FlowControl|Delay 1.1)
                    (Input|EnableInput _asbp_first_person_character 0)
                    (Rendering|SetVisibility (Variables|/Game/Konya/Blueprints/BP_FirstPersonCharacter.BP_FirstPersonCharacter_C|GetJump%20Scare%20Mesh _asbp_first_person_character) false false)
                    (Default|TeleporttoLatestCheckpoint _asbp_first_person_character)
                    (goto _label Reset)))))
            (else
              (Utilities|FlowControl|DoOnce false :!label _label_2
                (:Completed
                  (CallFunction|PlaySound "/Game/Konya/Audio/AI_Chasing.AI_Chasing")
                  (Utilities|FlowControl|Delay 2.91)
                  (goto _label_2 Reset))))))))
    (:then_1
      (Utilities|FlowControl|RetriggerableDelay 1.0)
      (CallFunction|RandomRoam))))

(event OnTargetPerceptionUpdated(AIPerception)
  (params (Actor :type Actor%20Object%20Reference) (Stimulus :type AI%20Stimulus%20Structure))
  (bind (_age _expirationage _strength _stimuluslocation _receiverlocation _tag _bsuccessfullysensed) (Utilities|Struct|BreakAIStimulus Stimulus))
  (Utilities|Casting|CastToBP_FirstPersonCharacter Actor)
  (if _bsuccessfullysensed
    (Variables|Default|SetInvestigating true)
    (AI|AIMoveTo self _stimuluslocation 0 5.0 false)))

(event Custom|Random%20Roam
  ;[0 0 0] Random Roam System
  (AI|AIMoveTo self (.RandomLocation (AI|Navigation|GetRandomReachablePointinRadius (Transformation|GetActorLocation) 1.5e+03 0 0)) 0 5.0 false
    (:OnSuccess
      (CallFunction|RandomRoam))))

(fn ConstructionScript
  (Utilities|FlowControl|DoOnce false
    (:Completed
      (Variables|Default|SetStart%20Location (Transformation|GetActorTransform))
      (bind _returnvalue (AddComponent|AddAudioComponent false))
      (Variables|Default|SetAudio%20Component _returnvalue))))

(fn PlaySound
  (params (Sound :type Sound%20Base%20Object%20Reference))
  (bind _audio_component (Variables|Default|GetAudio%20Component))
  (Audio|Components|Audio|SetSound _audio_component Sound)
  (Audio|Components|Audio|Play _audio_component 0.0))